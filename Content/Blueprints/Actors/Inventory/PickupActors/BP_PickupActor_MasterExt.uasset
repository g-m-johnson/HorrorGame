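; Base pickup actor that shows a prompt in the world and lets the player add its item to their inventory.
; UpdateWidget traces from the mesh to the player camera, showing the camera-facing prompt only when unobstructed.
; Within pickup distance it toggles the prompt and enables this actor's input; otherwise input is disabled.
; The action input adds the item to the character's inventory component, keeping any remainder or destroying the actor.
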(event `self.UpdateWidget`
  (bind _returnvalue (`GameplayStatics.GetPlayerController` 0))
  (bind _promptwidget (`self.PromptWidget`))
  (bind _promptwidget_2 (`self.PromptWidget`))
  (bind (_outhit _returnvalue_2) (`KismetSystemLibrary.LineTraceSingle` (`SceneComponent.K2_GetComponentLocation` (`self.StaticMesh`)) (`SceneComponent.K2_GetComponentLocation` (`FirstPersonCharacterBase.CameraComponent` (`self.PlayerRef`))) "TraceTypeQuery1"))
  (if (not _returnvalue_2)
    (`SceneComponent.SetVisibility` _promptwidget_2 true false)
    (`SceneComponent.K2_SetWorldRotation` _promptwidget (`KismetMathLibrary.FindLookAtRotation` (`SceneComponent.K2_GetComponentLocation` _promptwidget) (`SceneComponent.K2_GetComponentLocation` (`FirstPersonCharacterBase.CameraComponent` (`self.PlayerRef`)))) false false)
    (bind (_bblockinghit _binitialoverlap _time _distance _location _impactpoint _normal _impactnormal _physmat _hitactor _hitcomponent _hitbonename _bonename _hititem _elementindex _faceindex _tracestart _traceend) (`GameplayStatics.BreakHitResult` _outhit))
    (bind _returnvalue_3 (<= (`KismetMathLibrary.VSize` (- _tracestart _traceend)) (`self.PickUpDistance`)))
    (`/Game/UMG/Inventory/W_PickUpPrompt.TogglePrompt` (cast `/Game/UMG/Inventory/W_PickUpPrompt` (`WidgetComponent.GetUserWidgetObject` (`self.PromptWidget`)) :!pure true) _returnvalue_3)
    (if _returnvalue_3
      (`self.EnableInput` _returnvalue)
      (else
        (`self.DisableInput` _returnvalue)))
    (else
      (`SceneComponent.SetVisibility` _promptwidget_2 false false)
      (`self.DisableInput` (`GameplayStatics.GetPlayerController` 0)))))

(event `EnhancedInput|/Game/GameBlueprints/Input/IA_Action`
  (params (ActionValue :type Boolean) (ElapsedSeconds :type "Float (double-precision)") (TriggeredSeconds :type "Float (double-precision)") (InputAction :type "InputAction Object Reference" :default "/Game/GameBlueprints/Input/IA_Action.IA_Action"))
  (:`Started`
    (bind (_success _remainder) (`/Game/Blueprints/Components/BPC_Inventory.AddItem` (`/Game/GameBlueprints/Level1/BP_L1Character.BPC_Inventory` (cast `/Game/GameBlueprints/Level1/BP_L1Character` (`self.PlayerRef`) :!pure true)) (`self.Item`) (`self.Amount`)))
    (if _success
      (if (> _remainder 0)
        (set `self.Amount` _remainder)
        (else
          (`self.K2_DestroyActor`))))))

(fn `UserConstructionScript`)