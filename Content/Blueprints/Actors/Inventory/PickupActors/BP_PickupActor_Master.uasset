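; Base pickup actor that shows a world-space prompt above its mesh and lets the player collect its item into their inventory.
; Overlapping the sphere with BP_L1Character starts per-tick updates that trace to the player's camera, hiding the prompt when blocked.
; When unobstructed, the prompt faces the camera and toggles with pickup range, which also gates actor input.
; IA_Action adds the item through BPCInventory, keeping any remainder or destroying the actor.
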(event `self.ReceiveTick`
  (params (DeltaSeconds :type "Float (single-precision)"))
  (bind (_returnvalue_x _returnvalue_y _returnvalue_z) (`KismetMathLibrary.BreakVector` (`SceneComponent.K2_GetComponentLocation` (`self.StaticMesh`))))
  (`SceneComponent.K2_SetWorldLocation` (`self.PromptWidget`) (`KismetMathLibrary.MakeVector` _returnvalue_x _returnvalue_y (+ _returnvalue_z (`self.WidgetDistanceAboveMesh`))) false false)
  (if (`self.UpdateActor`)
    (`self.UpdateWidget`)))

(event `self.Sphere.OnComponentBeginOverlap`
  (params (OverlappedComponent :type "PrimitiveComponent Object Reference") (OtherActor :type "Actor Object Reference") (OtherComp :type "PrimitiveComponent Object Reference") (OtherBodyIndex :type Integer) (bFromSweep :type Boolean) (SweepResult :type "HitResult Structure (by ref)"))
  (bind _asbp_l1character (cast `/Game/GameBlueprints/Level1/BP_L1Character` OtherActor))
  (set `self.PlayerRef` _asbp_l1character)
  (`SceneComponent.SetVisibility` (`self.PromptWidget`) true false)
  (set `self.UpdateActor` true))

(event `self.Sphere.OnComponentEndOverlap`
  (params (OverlappedComponent :type "PrimitiveComponent Object Reference") (OtherActor :type "Actor Object Reference") (OtherComp :type "PrimitiveComponent Object Reference") (OtherBodyIndex :type Integer))
  (`SceneComponent.SetVisibility` (`self.PromptWidget`) false false)
  (set `self.UpdateActor` false)
  (`self.DisableInput` (`GameplayStatics.GetPlayerController` 0)))

(event `EnhancedInput|/Game/GameBlueprints/Input/IA_Action`
  (params (ActionValue :type Boolean) (ElapsedSeconds :type "Float (double-precision)") (TriggeredSeconds :type "Float (double-precision)") (InputAction :type "InputAction Object Reference" :default "/Game/GameBlueprints/Input/IA_Action.IA_Action"))
  (:`Started`
    (bind (_success _remainder) (`/Game/Blueprints/Components/BPC_Inventory.AddItem` (`/Game/GameBlueprints/Level1/BP_L1Character.BPC_Inventory` (`self.PlayerRef`)) (`self.Item`) (`self.Amount`)))
    (if _success
      (if (> _remainder 0)
        (set `self.Amount` _remainder)
        (else
          (`self.K2_DestroyActor`))))))

(fn `UpdateWidget`
  (bind _returnvalue (`GameplayStatics.GetPlayerController` 0))
  (bind _promptwidget (`self.PromptWidget`))
  (bind _promptwidget_2 (`self.PromptWidget`))
  (bind (_outhit _returnvalue_2) (`KismetSystemLibrary.LineTraceSingle` (`SceneComponent.K2_GetComponentLocation` (`self.StaticMesh`)) (`SceneComponent.K2_GetComponentLocation` (`/Game/GameBlueprints/Level1/BP_L1Character.Camera` (`self.PlayerRef`))) "TraceTypeQuery1"))
  (if (not _returnvalue_2)
    (`SceneComponent.SetVisibility` _promptwidget_2 true false)
    (`SceneComponent.K2_SetWorldRotation` _promptwidget (`KismetMathLibrary.FindLookAtRotation` (`SceneComponent.K2_GetComponentLocation` _promptwidget) (`SceneComponent.K2_GetComponentLocation` (`/Game/GameBlueprints/Level1/BP_L1Character.Camera` (`self.PlayerRef`)))) false false)
    (bind (_bblockinghit _binitialoverlap _time _distance _location _impactpoint _normal _impactnormal _physmat _hitactor _hitcomponent _hitbonename _bonename _hititem _elementindex _faceindex _tracestart _traceend) (`GameplayStatics.BreakHitResult` _outhit))
    (bind _returnvalue_3 (<= (`KismetMathLibrary.VSize` (- _tracestart _traceend)) (`self.PickUpDistance`)))
    (`/Game/UMG/Inventory/W_PickUpPrompt.TogglePrompt` (cast `/Game/UMG/Inventory/W_PickUpPrompt` (`WidgetComponent.GetUserWidgetObject` (`self.PromptWidget`)) :!pure true) _returnvalue_3)
    (if _returnvalue_3
      (`self.EnableInput` _returnvalue)
      (else
        (`self.DisableInput` _returnvalue)))
    (else
      (`SceneComponent.SetVisibility` _promptwidget_2 false false)
      (`self.DisableInput` (`GameplayStatics.GetPlayerController` 0)))))

(fn `UserConstructionScript`
  (`SceneComponent.K2_SetRelativeLocation` (`self.PromptWidget`) (`KismetMathLibrary.MakeVector` 0.0 0.0 (`self.WidgetDistanceAboveMesh`)) false false))