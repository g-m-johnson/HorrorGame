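; BP_InventoryItem_Bandage is an inventory item that heals the player when used.
; UseItem casts PlayerRef to BP_L1Character and compares its health component's current health against the maximum.
; Below maximum, it adds AmountOfHealth and sets UseItemSuccess to true; at full health it leaves health unchanged and reports failure.
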(event `self.UseItem`
  (bind _component_health (`/Game/GameBlueprints/Level1/BP_L1Character.Component_Health` (cast `/Game/GameBlueprints/Level1/BP_L1Character` (`self.PlayerRef`) :!pure true)))
  (if (< (`Component_Health.CurrentHealth` _component_health) (`Component_Health.MaxHealth` _component_health))
    (`Component_Health.AddHealth` _component_health (`self.AmountOfHealth`))
    (set `self.UseItemSuccess` true)
    (else
      (set `self.UseItemSuccess` false))))

(fn `UserConstructionScript`)