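; BP_Interaction_Door is an interactable door actor that swings open and closed.
; Each Interact event flips the IsDoorClosed flag and plays or reverses the OpenDoorTL timeline.
; The timeline's Alpha drives a lerp on the Door component's relative yaw, rotating it a quarter turn between closed and open.
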(event `/Game/Blueprints/Interfaces/BPI_Interaction.Interact`
  (if (`self.IsDoorClosed`)
    (set `self.IsDoorClosed` false)
    (bind (_direction _alpha) (`Timeline|OpenDoorTL` :!label _label)
      (:`Update`
        (`SceneComponent.K2_SetRelativeRotation` (`self.Door`) (`KismetMathLibrary.MakeRotator` 0.0 0.0 (`KismetMathLibrary.Lerp` 0.0 -90.0 _alpha)) false false)))
    (else
      (set `self.IsDoorClosed` true)
      (goto _label :!via `Reverse`))))

(fn `UserConstructionScript`
  (`parent.UserConstructionScript`))