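; Inventory component that stores item classes and amounts in a slot array sized from the player controller.
; AddItem recursively fills partial stacks, then empty slots, returning any remainder, and each change refreshes the matching grid widget slot.
; UseItem runs the item actor's UseItem and removes one on success; DropItem empties the slot and spawns a physics pickup along a camera trace.
; It also expands slots and opens an examination widget.
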(event `self.ReceiveBeginPlay`
  (`self.Initialise`))

(event `Initialise`
  (bind _asbp_player_controller (cast `/Game/GameBlueprints/BP_PlayerController` (`GameplayStatics.GetPlayerController` 0) :!pure true))
  (`KismetArrayLibrary.Array_Resize` (`self.InventorySlots`) (`/Game/GameBlueprints/BP_PlayerController.InventorySlots` _asbp_player_controller))
  (set `self.W_InventoryMenuRef` (`/Game/GameBlueprints/BP_PlayerController.InventoryMenuRef` _asbp_player_controller))
  (bind _asbp_l1character (cast `/Game/GameBlueprints/Level1/BP_L1Character` (`GameplayStatics.GetPlayerCharacter` 0)))
  (set `self.PlayerRef` _asbp_l1character)
  (bind _returnvalue (`|CreateWidget` "/Game/UMG/Inventory/W_Examination.W_Examination_C" null null))
  (set `self.WExaminationRef` _returnvalue)
  (set `/Game/GameBlueprints/BP_PlayerController.WExaminationWIdgetRef` (`self.WExaminationRef`) _asbp_player_controller)
  (bind _outactors (`GameplayStatics.GetAllActorsOfClass` "/Game/Blueprints/Actors/Inventory/BP_Examination.BP_Examination_C"))
  (set `self.BPExaminationRef` (`|GetArrayItem` _outactors))
  (set `/Game/UMG/Inventory/W_Examination.BPCInventoryRef` self (`self.WExaminationRef`)))

(event `CreateExaminationWidget`
  (params (Index :type Integer))
  (bind _w_inventorymenuref (`self.W_InventoryMenuRef`))
  (`/Game/UMG/Inventory/W_Examination.UpdateWidget` (`self.WExaminationRef`) Index)
  (`Widget.SetVisibility` _w_inventorymenuref "Collapsed")
  (`/Engine/EditorBlueprintResources/StandardMacros.IsValid` (`/Game/UMG/Inventory/W_InventoryMenu.W_InventoryDropDown` _w_inventorymenuref)
    (:`Is Valid`
      (`/Game/UMG/Inventory/W_InventoryMenu.CloseDropDownMenu` _w_inventorymenuref))
    (:`Is Not Valid`
      _))
  (`UserWidget.AddToViewport` (`self.WExaminationRef`) 2)
  (set `/Game/GameBlueprints/BP_PlayerController.IsInventoryOpen` false (cast `/Game/GameBlueprints/BP_PlayerController` (`GameplayStatics.GetPlayerController` 0) :!pure true)))

(fn `AddItem`
  (params (Item :type "InventoryItem_Master Class Reference") (Amount :type Integer))
  (returns (Success :type Boolean) (Remainder :type Integer))
  (locals (LocalItem :type "InventoryItem_Master Class Reference") (`Local Amount` :type Integer) (LocalMaxStackAmount :type Integer) (LocalIndex :type Integer :default 0))
  (bind (_success _index) (`self.CheckForEmptySlot`))
  (bind (_success_2 _index_2) (`self.CheckForEmptySlot`))
  (bind _localindex (`local.LocalIndex`))
  (bind _returnvalue (- (`local.Local Amount`) 1))
  (bind (_itemname _icon _itemdescription _maxstackamount) (break `ItemData` (defaults `Object` (`local.LocalItem`))))
  (bind _returnvalue_2 (+ (`.Amount` (`self.GetItemDataAtIndex` (`local.LocalIndex`))) (`local.Local Amount`)))
  (set `local.LocalItem` Item)
  (set `local.Local Amount` Amount)
  (set `local.LocalMaxStackAmount` _maxstackamount)
  (if (> _maxstackamount 1)
    (bind (_success_3 _index_3) (`self.CheckForFreeSlot` (`local.LocalItem`)))
    (if _success_3
      (set `local.LocalIndex` _index_3) ; Set local index to index of stackable slot
      (if (> _returnvalue_2 (`local.LocalMaxStackAmount`))
        (set `local.Local Amount` (- _returnvalue_2 (`local.LocalMaxStackAmount`)))
        (`KismetArrayLibrary.Array_Set` (`self.InventorySlots`) (`local.LocalIndex`) (make `InventoryItem` (`local.LocalItem`) (`local.LocalMaxStackAmount`)))
        (`self.UpdateInventorySlot` (`local.LocalIndex`))
        (bind (_success_4 _remainder) (`self.AddItem` (`local.LocalItem`) (`local.Local Amount`)))
        (return true _remainder)
        (else
          (`KismetArrayLibrary.Array_Set` (`self.InventorySlots`) (`local.LocalIndex`) (make `InventoryItem` (`local.LocalItem`) _returnvalue_2))
          (`self.UpdateInventorySlot` (`local.LocalIndex`))
          (return true 0) ; All items added successfully
        ))
      (elif _success
        (set `local.LocalIndex` _index) ; Set local index to index of empty slot
        (if (> (`local.Local Amount`) (`local.LocalMaxStackAmount`))
          (`KismetArrayLibrary.Array_Set` (`self.InventorySlots`) (`local.LocalIndex`) (make `InventoryItem` (`local.LocalItem`) (`local.LocalMaxStackAmount`)))
          (`self.UpdateInventorySlot` _localindex)
          (bind (_success_5 _remainder_2) (`self.AddItem` (`local.LocalItem`) (- (`local.Local Amount`) (`local.LocalMaxStackAmount`)))) ; Add the rest of the items that do not fit into this slot
          (return true _remainder_2) ; Added item, some may be remaining
          (else
            (`KismetArrayLibrary.Array_Set` (`self.InventorySlots`) (`local.LocalIndex`) (make `InventoryItem` (`local.LocalItem`) (`local.Local Amount`))) ; Add item to inventory slots array
            (`self.UpdateInventorySlot` _localindex) ; Update inventory
            (return true 0) ; Added item(s), nothing more to add
          ))
        (else
          (return false (`local.Local Amount`)) ; Unable to add any items
        )))
    (elif _success_2
      (bind _output_get (set `local.LocalIndex` _index_2)) ; Set LocalIndex to index of free slot
      (`KismetArrayLibrary.Array_Set` (`self.InventorySlots`) _output_get (make `InventoryItem` (`local.LocalItem`) 1)) ; Set inventory slot to item at correct index
      (`self.UpdateInventorySlot` (`local.LocalIndex`)) ; Update inventory at slot
      (if (> _returnvalue 0)
        (bind (_success_6 _remainder_3) (`self.AddItem` (`local.LocalItem`) _returnvalue)) ; Keep calling function until all items have been stored/no more slots
        (return true _remainder_3) ; Added item, some remaining though
        (else
          (return true 0) ; Found empty slot, nothing more to add
        ))
      (else
        (`KismetSystemLibrary.PrintString` "No free slots")
        (return false (`local.Local Amount`)) ; Unable to find empty slot
      ))))

(fn `AddMoreSlots`
  (params (Amount :type Integer))
  (bind _w_inventorymenuref (`self.W_InventoryMenuRef`))
  (bind _asbp_player_controller (cast `/Game/GameBlueprints/BP_PlayerController` (`GameplayStatics.GetPlayerController` 0) :!pure true))
  (bind _w_inventorygrid (`/Game/UMG/Inventory/W_InventoryMenu.W_InventoryGrid` _w_inventorymenuref))
  (bind _output_get (set `/Game/GameBlueprints/BP_PlayerController.InventorySlots` (+ (`/Game/GameBlueprints/BP_PlayerController.InventorySlots` _asbp_player_controller) Amount) _asbp_player_controller))
  (`KismetArrayLibrary.Array_Resize` (`self.InventorySlots`) _output_get)
  (`/Game/UMG/Inventory/W_InventoryGrid.AddMoreSlots` _w_inventorygrid Amount)
  (for _array_element (`/Game/UMG/Inventory/W_InventoryGrid.SlotsArray` _w_inventorygrid)
    (`/Game/UMG/Inventory/W_InventorySlot.Initialise` _array_element _w_inventorymenuref)))

(fn `CheckForEmptySlot`
  (returns (Success :type Boolean) (Index :type Integer))
  (locals (LocalSuccess :type Boolean) (LocalIndex :type Integer))
  (for (_array_element _array_index) (`self.InventorySlots`)
    (if (`KismetSystemLibrary.IsValidClass` (`.Item` (break `InventoryItem` _array_element)))
      (set `local.LocalSuccess` false)
      (else
        (set `local.LocalSuccess` true)
        (set `local.LocalIndex` _array_index)
        (break))))
  (return (`local.LocalSuccess`) (`local.LocalIndex`)))

(fn `CheckForFreeSlot`
  (params (Item :type "InventoryItem_Master Class Reference"))
  (returns (Success :type Boolean) (Index :type Integer))
  (locals (LocalSuccess :type Boolean) (LocalIndex :type Integer))
  (for (_array_element _array_index) (`self.InventorySlots`)
    (bind (_item _amount) (break `InventoryItem` _array_element))
    (if (and (== _item Item) (< _amount (`.MaxStackAmount` (break `ItemData` (defaults `Object` Item)))))
      (set `local.LocalSuccess` true)
      (set `local.LocalIndex` _array_index)
      (break)
      (else
        (set `local.LocalSuccess` false))))
  (return (`local.LocalSuccess`) (`local.LocalIndex`)))

(fn `DropItem`
  (params (Index :type Integer))
  (locals (LocalIndex :type Integer) (LocalAmount :type Integer :default 0) (LocalItem :type "InventoryItem_Master Class Reference"))
  (bind _cameracomponent (`FirstPersonCharacterBase.CameraComponent` (`self.PlayerRef`)))
  (bind _returnvalue (`SceneComponent.K2_GetComponentLocation` _cameracomponent))
  (bind _output_get (set `local.LocalIndex` Index))
  (bind (_item _amount) (`self.GetItemDataAtIndex` _output_get))
  (set `local.LocalItem` _item)
  (bind _output_get_2 (set `local.LocalAmount` _amount))
  (if (> _output_get_2 0)
    (for _ (range (`local.LocalAmount`))
      (`self.RemoveItem` (`local.LocalIndex`)))
    (`/Game/UMG/Inventory/W_InventoryMenu.CloseDropDownMenu` (`self.W_InventoryMenuRef`))
    (bind (_outhit _returnvalue_2) (`KismetSystemLibrary.LineTraceSingle` _returnvalue (+ _returnvalue (* (`SceneComponent.GetForwardVector` _cameracomponent) 200.0)) "TraceTypeQuery1"))
    (bind (_bblockinghit _binitialoverlap _time _distance _location _impactpoint _normal _impactnormal _physmat _hitactor _hitcomponent _hitbonename _bonename _hititem _elementindex _faceindex _tracestart _traceend) (`GameplayStatics.BreakHitResult` _outhit))
    (bind _returnvalue_3 (`|SpawnActorFromClass` (`.PickupActor` (break `ItemData` (defaults `Object` (`local.LocalItem`)))) (`KismetMathLibrary.MakeTransform` (select `bool` _returnvalue_2 :`false` _traceend :`true` _tracestart)) "Undefined" "MultiplyWithRoot" null null))
    (bind _asbp_pickup_actor_master_ext (cast `/Game/Blueprints/Actors/Inventory/PickupActors/BP_PickupActor_MasterExt` _returnvalue_3 :!pure true))
    (set `PickupActor_Master.Amount` (`local.LocalAmount`) _asbp_pickup_actor_master_ext)
    (`PrimitiveComponent.SetSimulatePhysics` (`PickupActor_Master.StaticMesh` _asbp_pickup_actor_master_ext) true)))

(fn `GetItemDataAtIndex`
  (params (Index :type Integer))
  (returns (Item :type "InventoryItem_Master Class Reference") (Amount :type Integer))
  (bind (_item _amount) (break `InventoryItem` (`|GetArrayItem` (`self.InventorySlots`) Index)))
  (return (castclass `InventoryItem_Master` _item :!pure true) _amount))

(fn `RemoveItem`
  (params (Index :type Integer))
  (locals (LocalIndex :type Integer))
  (bind (_item _amount) (`self.GetItemDataAtIndex` Index))
  (set `local.LocalIndex` Index)
  (if (> _amount 1)
    (`KismetArrayLibrary.Array_Set` (`self.InventorySlots`) (`local.LocalIndex`) (make `InventoryItem` _item (- _amount 1)))
    (else
      (`KismetArrayLibrary.Array_Set` (`self.InventorySlots`) (`local.LocalIndex`) (make `InventoryItem` null))))
  (`self.UpdateInventorySlot` (`local.LocalIndex`)))

(fn `UpdateInventorySlot`
  (params (Index :type Integer))
  (`/Game/UMG/Inventory/W_InventorySlot.UpdateSlot` (`|GetArrayItem` (`/Game/UMG/Inventory/W_InventoryGrid.SlotsArray` (`/Game/UMG/Inventory/W_InventoryMenu.W_InventoryGrid` (`/Game/GameBlueprints/BP_PlayerController.InventoryMenuRef` (cast `/Game/GameBlueprints/BP_PlayerController` (`GameplayStatics.GetPlayerController` 0) :!pure true)))) Index)))

(fn `UseItem`
  (params (Index :type Integer))
  (locals (LocalIndex :type Integer))
  (bind _output_get (set `local.LocalIndex` Index))
  (bind (_item _amount) (`self.GetItemDataAtIndex` _output_get))
  (if (> _amount 0)
    (bind _returnvalue (`GameplayStatics.GetActorOfClass` _item))
    (`/Engine/EditorBlueprintResources/StandardMacros.IsValid` _returnvalue
      (:`Is Valid`
        (`InventoryItem_Master.UseItem` _returnvalue)
        (if (`InventoryItem_Master.UseItemSuccess` _returnvalue)
          (`self.RemoveItem` (`local.LocalIndex`) :!label _label)
          (`/Game/UMG/Inventory/W_InventoryMenu.CloseDropDownMenu` (`self.W_InventoryMenuRef`))
          (else
            (`KismetSystemLibrary.PrintString` "Use item not successful" :!label _label_2))))
      (:`Is Not Valid`
        (bind _returnvalue_2 (`|SpawnActorFromClass` _item (`KismetMathLibrary.MakeTransform` (0.0 0.0 0.0)) "Undefined" "MultiplyWithRoot" null null))
        (`InventoryItem_Master.UseItem` _returnvalue_2)
        (if (`InventoryItem_Master.UseItemSuccess` _returnvalue_2)
          (goto _label)
          (else
            (goto _label_2)))))))