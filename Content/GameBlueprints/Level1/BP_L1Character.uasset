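; First-person player character for Level 1 that maps Enhanced Input to walking, jumping, sprinting, crouching, flashlight, interaction and grabbing.
; Movement and flashlight components are initialised at BeginPlay alongside the HUD, with a reversible timeline resizing the capsule for crouch.
; Camera line traces send BPI_Interaction and BPI_Grab messages to hit actors, and speed selects walk or run head-bob shakes.
; Debug prints show battery each tick, and number keys test inventory and health.
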(event `self.ShortenPlayerCapsule`
  (bind (_direction _alpha) (`Timeline|Timeline` :!label _label)
    (:`Update`
      (`CapsuleComponent.SetCapsuleHalfHeight` (`self.CapsuleComponent`) (`KismetMathLibrary.Lerp` 88.0 (`Component_Movement.CrouchHalfHeight` (`self.BPC_Movement`)) _alpha) true))))

(event `self.ReceiveBeginPlay`
  (bind _asbp_player_controller (cast `/Game/GameBlueprints/BP_PlayerController` (`self.GetController`)))
  (`EnhancedInputSubsystemInterface.AddMappingContext` (pcsubsystem `EnhancedInputLocalPlayerSubsystem` _asbp_player_controller) "/Game/GameBlueprints/Input/IMC_Player.IMC_Player" 0 (struct))
  (`self.Initialise`))

(event `self.LengthenPlayerCapsule`
  (goto _label :!via `Reverse`))

(event `EnhancedInput|/Game/GameBlueprints/Input/IA_WalkForward`
  (params (ActionValue :type "Float (double-precision)") (ElapsedSeconds :type "Float (double-precision)") (TriggeredSeconds :type "Float (double-precision)") (InputAction :type "InputAction Object Reference" :default "/Game/GameBlueprints/Input/IA_WalkForward.IA_WalkForward"))
  ;[1 0.9298 0.1725] Moving
  (:`Triggered`
    (`self.AddMovementInput` (`self.GetActorForwardVector`) ActionValue :!label _label_2)
    (`self.HeadBob`))
  (:`Started`
    (goto _label_2)))

(event `EnhancedInput|/Game/GameBlueprints/Input/IA_Action`
  (params (ActionValue :type Boolean) (ElapsedSeconds :type "Float (double-precision)") (TriggeredSeconds :type "Float (double-precision)") (InputAction :type "InputAction Object Reference" :default "/Game/GameBlueprints/Input/IA_Action.IA_Action"))
  (:`Started`
    (bind _hitactor (`self.LineTrace` 350.0))
    (if (and (`KismetSystemLibrary.IsValid` _hitactor) (`KismetSystemLibrary.DoesImplementInterface` _hitactor "/Game/Blueprints/Interfaces/BPI_Interaction.BPI_Interaction_C"))
      (message `/Game/Blueprints/Interfaces/BPI_Interaction.Interact` _hitactor))))

(event `EnhancedInput|/Game/GameBlueprints/Input/IA_StrafeRight`
  (params (ActionValue :type "Float (double-precision)") (ElapsedSeconds :type "Float (double-precision)") (TriggeredSeconds :type "Float (double-precision)") (InputAction :type "InputAction Object Reference" :default "/Game/GameBlueprints/Input/IA_StrafeRight.IA_StrafeRight"))
  ;[1 0.9298 0.1725] Moving
  (:`Triggered`
    (`self.AddMovementInput` (`self.GetActorRightVector`) ActionValue :!label _label_3)
    (`self.HeadBob`))
  (:`Started`
    (goto _label_3)))

(event `EnhancedInput|/Game/GameBlueprints/Input/IA_LMB`
  (params (ActionValue :type Boolean) (ElapsedSeconds :type "Float (double-precision)") (TriggeredSeconds :type "Float (double-precision)") (InputAction :type "InputAction Object Reference" :default "/Game/GameBlueprints/Input/IA_LMB.IA_LMB"))
  (bind _grabbedobject (`self.GrabbedObject`))
  (:`Started`
    (bind _hitactor (`self.LineTrace` 350.0))
    (set `self.GrabbedObject` _hitactor)
    (if (and (`KismetSystemLibrary.IsValid` _hitactor) (`KismetSystemLibrary.DoesImplementInterface` _hitactor "/Game/Blueprints/Interfaces/BPI_Grab.BPI_Grab_C"))
      (message `/Game/Blueprints/Interfaces/BPI_Grab.GrabObject` (`self.GrabbedObject`))))
  (:`Completed`
    (`/Engine/EditorBlueprintResources/StandardMacros.IsValid` _grabbedobject
      (:`Is Valid`
        (message `/Game/Blueprints/Interfaces/BPI_Grab.ReleaseObject` _grabbedobject)
        (set `self.GrabbedObject` null)))))

(event `EnhancedInput|/Game/GameBlueprints/Input/IA_Jump`
  (params (ActionValue :type Boolean) (ElapsedSeconds :type "Float (double-precision)") (TriggeredSeconds :type "Float (double-precision)") (InputAction :type "InputAction Object Reference" :default "/Game/GameBlueprints/Input/IA_Jump.IA_Jump"))
  ;[1 0.9298 0.1725] Moving
  (:`Triggered`
    (`self.Jump` :!label _label_4))
  (:`Started`
    (goto _label_4))
  (:`Completed`
    (`self.StopJumping`)))

(event `EnhancedInput|/Game/GameBlueprints/Input/IA_Sprint`
  (params (ActionValue :type Boolean) (ElapsedSeconds :type "Float (double-precision)") (TriggeredSeconds :type "Float (double-precision)") (InputAction :type "InputAction Object Reference" :default "/Game/GameBlueprints/Input/IA_Sprint.IA_Sprint"))
  (bind _bpc_movement (`self.BPC_Movement`))
  ;[1 0.9298 0.1725] Moving
  (:`Started`
    (`Component_Movement.StartSprint` _bpc_movement))
  (:`Completed`
    (`Component_Movement.StopSprint` _bpc_movement)))

(event `self.ReceiveTick`
  (params (DeltaSeconds :type "Float (single-precision)"))
  (`KismetSystemLibrary.PrintString` (`KismetStringLibrary.Conv_DoubleToString` (`Component_Flashlight.CurrentBatteryLevel` (`self.Component_Flashlight`))) true true (struct :`R` 1.0 :`G` 0.284819 :`A` 1.0) DeltaSeconds))

(event `EnhancedInput|/Game/GameBlueprints/Input/IA_Flashlight`
  (params (ActionValue :type Boolean) (ElapsedSeconds :type "Float (double-precision)") (TriggeredSeconds :type "Float (double-precision)") (InputAction :type "InputAction Object Reference" :default "/Game/GameBlueprints/Input/IA_Flashlight.IA_Flashlight"))
  (:`Started`
    (`Component_Flashlight.ToggleFlashlight` (`self.Component_Flashlight`))))

(event `EnhancedInput|/Game/GameBlueprints/Input/IA_Crouch`
  (params (ActionValue :type Boolean) (ElapsedSeconds :type "Float (double-precision)") (TriggeredSeconds :type "Float (double-precision)") (InputAction :type "InputAction Object Reference" :default "/Game/GameBlueprints/Input/IA_Crouch.IA_Crouch"))
  (bind _bpc_movement (`self.BPC_Movement`))
  (:`Started`
    (if (`Component_Movement.bIsCrouching` _bpc_movement)
      (`Component_Movement.EndCrouch` _bpc_movement)
      (else
        (`Component_Movement.StartCrouch` _bpc_movement)))))

(event `Key|One`
  (params (Key :type "Key Structure"))
  (:`Pressed`
    (for _array_element (`/Game/Blueprints/Components/BPC_Inventory.InventorySlots` (`self.BPC_Inventory`))
      (bind (_item _amount) (break `InventoryItem` _array_element))
      (`KismetSystemLibrary.PrintString` (`KismetMathLibrary.SelectString` (`KismetStringLibrary.Concat_StrStr` (`KismetSystemLibrary.GetClassDisplayName` _item) ": " (`KismetStringLibrary.Conv_IntToString` _amount)) "no item" (`KismetSystemLibrary.IsValidClass` null))))))

(event `Key|Two`
  (params (Key :type "Key Structure"))
  (bind _component_health (`self.Component_Health`))
  (:`Pressed`
    (`Component_Health.RemoveHealth` _component_health 25.0)
    (`KismetSystemLibrary.PrintString` (`KismetStringLibrary.Conv_DoubleToString` (`Component_Health.CurrentHealth` _component_health)))))

(event `Key|Three`
  (params (Key :type "Key Structure"))
  (bind _component_health (`self.Component_Health`))
  (:`Pressed`
    (`Component_Health.AddHealth` _component_health 25.0)
    (`KismetSystemLibrary.PrintString` (`KismetStringLibrary.Conv_DoubleToString` (`Component_Health.CurrentHealth` _component_health)))))

(fn `HeadBob`
  (bind _returnvalue (`KismetMathLibrary.VSize` (`self.GetVelocity`)))
  (bind _playercameramanager (`PlayerController.PlayerCameraManager` (`GameplayStatics.GetPlayerController` 0)))
  (bind _returnvalue_2 (`KismetMathLibrary.MapRangeClamped` (`KismetMathLibrary.VSize` (`self.GetVelocity`)) 0.0 (`CharacterMovementComponent.MaxWalkSpeed` (`self.CharacterMovement`)) 0.0 1.0))
  (if (and (>= _returnvalue (`Component_Movement.WalkSpeed` (`self.BPC_Movement`))) (not (`NavMovementComponent.IsFalling` (`self.CharacterMovement`))))
    (if (and (>= _returnvalue (`Component_Movement.SprintSpeed` (`self.BPC_Movement`))) (not (`NavMovementComponent.IsFalling` (`self.CharacterMovement`))))
      (`PlayerCameraManager.StartCameraShake` :`self` _playercameramanager :`ShakeClass` "/Game/Blueprints/CameraShakes/CS_HeadBob_Run.CS_HeadBob_Run_C" :`Scale` _returnvalue_2)
      (else
        (`PlayerCameraManager.StartCameraShake` :`self` _playercameramanager :`ShakeClass` "/Game/Blueprints/CameraShakes/CS_HeadBob_Walk.CS_HeadBob_Walk_C" :`Scale` _returnvalue_2)))))

(fn `Initialise`
  (`|ExecutionSequence`
    (:`then_0`
      (`Component_Movement.Initialise` (`self.BPC_Movement`) self)
      (`Component_Flashlight.Initialise` (`self.Component_Flashlight`) self))
    (:`then_1`
      (bind _returnvalue (`|CreateWidget` "/Game/UMG/W_MainHUD.W_MainHUD_C" null self))
      (bind _output_get (set `self.MainHUDRef` _returnvalue))
      (`UserWidget.AddToViewport` _output_get 0))))

(fn `LineTrace`
  (params (Length :type "Float (double-precision)") (DrawDebugType :type "EDrawDebugTrace Enum" :default "None"))
  (returns (HitActor :type "Actor Object Reference"))
  (bind _cameracomponent (`self.CameraComponent`))
  (bind _returnvalue (`SceneComponent.K2_GetComponentLocation` _cameracomponent))
  (bind _outhit (`KismetSystemLibrary.LineTraceSingle` :`Start` _returnvalue :`End` (+ _returnvalue (* (`SceneComponent.GetForwardVector` _cameracomponent) Length)) :`TraceChannel` "TraceTypeQuery1" :`DrawDebugType` DrawDebugType))
  (return (`.HitActor` (`GameplayStatics.BreakHitResult` _outhit))))

(fn `UserConstructionScript`)