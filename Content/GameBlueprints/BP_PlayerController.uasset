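; Player controller that handles camera look input and opens and closes the inventory menu.
; On BeginPlay it creates the W_InventoryMenu widget collapsed in the viewport, and look inputs apply pitch and yaw scaled by LookSensitivity.
; The inventory toggle flips IsPaused, disabling or restoring character movement and look, and switches cursor, menu visibility and input mode without actually pausing the game.
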(event `self.ReceiveBeginPlay`
  (bind _returnvalue (`|CreateWidget` "/Game/UMG/Inventory/W_InventoryMenu.W_InventoryMenu_C"))
  (bind _output_get (set `self.InventoryMenuRef` _returnvalue))
  (`Widget.SetVisibility` _output_get "Collapsed")
  (`UserWidget.AddToViewport` _output_get 0))

(event `EnhancedInput|/Game/GameBlueprints/Input/IA_LookUp`
  (params (ActionValue :type "Float (double-precision)") (ElapsedSeconds :type "Float (double-precision)") (TriggeredSeconds :type "Float (double-precision)") (InputAction :type "InputAction Object Reference" :default "/Game/GameBlueprints/Input/IA_LookUp.IA_LookUp"))
  ;[0.6621 1 0.3574] Looking
  (:`Triggered`
    (`self.AddPitchInput` (* ActionValue (`self.LookSensitivity`)))))

(event `EnhancedInput|/Game/GameBlueprints/Input/IA_LookRight`
  (params (ActionValue :type "Float (double-precision)") (ElapsedSeconds :type "Float (double-precision)") (TriggeredSeconds :type "Float (double-precision)") (InputAction :type "InputAction Object Reference" :default "/Game/GameBlueprints/Input/IA_LookRight.IA_LookRight"))
  ;[0.6621 1 0.3574] Looking
  (:`Triggered`
    (`self.AddYawInput` (* ActionValue (`self.LookSensitivity`)))))

(event `EnhancedInput|/Game/GameBlueprints/Input/IA_InventoryToggle`
  (params (ActionValue :type Boolean) (ElapsedSeconds :type "Float (double-precision)") (TriggeredSeconds :type "Float (double-precision)") (InputAction :type "InputAction Object Reference" :default "/Game/GameBlueprints/Input/IA_InventoryToggle.IA_InventoryToggle"))
  (:`Started`
    (`self.ToggleInventory`)))

(event `ToggleInventory`
  (bind _inventorymenuref (`self.InventoryMenuRef`))
  (bind _charactermovement (`Character.CharacterMovement` (`GameplayStatics.GetPlayerCharacter` 0)))
  (if (`self.IsPaused`)
    (set `self.IsPaused` false)
    (`CharacterMovementComponent.SetMovementMode` _charactermovement "MOVE_Walking" 0)
    (`self.ResetIgnoreLookInput`)
    (set `self.bShowMouseCursor` false)
    (`Widget.SetVisibility` _inventorymenuref "Collapsed")
    (`WidgetBlueprintLibrary.SetInputMode_GameOnly` self)
    (else
      (set `self.IsPaused` true)
      (`CharacterMovementComponent.DisableMovement` _charactermovement)
      (`self.SetIgnoreLookInput` true)
      (set `self.bShowMouseCursor` true)
      (`Widget.SetVisibility` _inventorymenuref "SelfHitTestInvisible")
      (`WidgetBlueprintLibrary.SetInputMode_GameAndUIEx` self _inventorymenuref))))

(fn `UserConstructionScript`)